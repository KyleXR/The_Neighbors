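; BP_DownstairsBasementDoor is an interactable door that takes the player to FirstFloorLevel.
; Interacting plays a door sound, saves through BP_GameMode, passes the level name to its ChangeLevel, then opens that level.
; A Box trigger toggles a Widget: any overlap shows it, while only BP_FirstPersonCharacter leaving hides it.
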(event OnComponentEndOverlap(Box)
  (params (OverlappedComponent :type Primitive%20Component%20Object%20Reference) (OtherActor :type Actor%20Object%20Reference) (OtherComp :type Primitive%20Component%20Object%20Reference) (OtherBodyIndex :type Integer))
  (Utilities|Casting|CastToBP_FirstPersonCharacter OtherActor)
  (Development|SetHiddeninGame (Variables|Default|GetWidget) true false))

(event OnComponentBeginOverlap(Box)
  (params (OverlappedComponent :type Primitive%20Component%20Object%20Reference) (OtherActor :type Actor%20Object%20Reference) (OtherComp :type Primitive%20Component%20Object%20Reference) (OtherBodyIndex :type Integer) (bFromSweep :type Boolean) (SweepResult :type Hit%20Result%20Structure%20%28by%20ref%29))
  (Development|SetHiddeninGame (Variables|Default|GetWidget) false false))

(event EventInteract
  (Audio|PlaySound2D "/Game/Game/Audio/Door_Open.Door_Open" 1.0 1.0 0.0 0 0)
  (bind _asbp_game_mode (Utilities|Casting|CastToBP_GameMode (Game|GetGameMode)))
  (Default|SaveGame _asbp_game_mode)
  (Default|ChangeLevel _asbp_game_mode "FirstFloorLevel")
  (Game|OpenLevel(byName) "FirstFloorLevel"))

(fn ConstructionScript)