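; BP_Checkpoint is a trigger actor that saves the game when the first-person character overlaps its Box.
; On overlap it loads the "Save1" slot, adds itself to the BP_Save CheckpointUsed collection, writes the slot back, then calls SaveGame on BP_GameMode.
; It does nothing if that slot fails to load as BP_Save.
; BeginPlay checks whether this checkpoint was already used, but takes no action on the result.
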(event OnComponentBeginOverlap(Box)
  (params (OverlappedComponent :type Primitive%20Component%20Object%20Reference) (OtherActor :type Actor%20Object%20Reference) (OtherComp :type Primitive%20Component%20Object%20Reference) (OtherBodyIndex :type Integer) (bFromSweep :type Boolean) (SweepResult :type Hit%20Result%20Structure%20%28by%20ref%29))
  (Utilities|Casting|CastToBP_FirstPersonCharacter OtherActor)
  (bind _returnvalue (SaveGame|LoadGamefromSlot "Save1"))
  (bind _asbp_save (Utilities|Casting|CastToBP_Save _returnvalue))
  (Utilities|Array|Add (Variables|/Game/Game/Blueprints/Save/BP_Save.BP_Save_C|GetCheckpointUsed _asbp_save) self)
  (SaveGame|SaveGametoSlot _asbp_save "Save1")
  (bind _asbp_game_mode (Utilities|Casting|CastToBP_GameMode (Game|GetGameMode)))
  (Default|SaveGame _asbp_game_mode))

(event EventBeginPlay
  (bind _returnvalue (SaveGame|LoadGamefromSlot "Save1"))
  (bind _asbp_save (Utilities|Casting|CastToBP_Save _returnvalue))
  (if (Utilities|Array|ContainsItem (Variables|/Game/Game/Blueprints/Save/BP_Save.BP_Save_C|GetCheckpointUsed _asbp_save) self)
    _))

(fn ConstructionScript)