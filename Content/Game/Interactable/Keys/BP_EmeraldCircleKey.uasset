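; Emerald circle key pickup that gives the first-person character the emerald key when interacted with.
; Interact sets HasEmeraldKey, plays a pickup sound and destroys the actor.
; A box overlap shows a widget and text prompt for any actor, but hides them only when the character leaves.
; The character reference is cached on end overlap, so Interact falls back to player character 0 when it is invalid.
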(event OnComponentBeginOverlap(Box)
  (params (OverlappedComponent :type Primitive%20Component%20Object%20Reference) (OtherActor :type Actor%20Object%20Reference) (OtherComp :type Primitive%20Component%20Object%20Reference) (OtherBodyIndex :type Integer) (bFromSweep :type Boolean) (SweepResult :type Hit%20Result%20Structure%20%28by%20ref%29))
  (Development|SetHiddeninGame (Variables|Default|GetWidget) false false))

(event OnComponentEndOverlap(Box)
  (params (OverlappedComponent :type Primitive%20Component%20Object%20Reference) (OtherActor :type Actor%20Object%20Reference) (OtherComp :type Primitive%20Component%20Object%20Reference) (OtherBodyIndex :type Integer))
  (bind _asbp_first_person_character (Utilities|Casting|CastToBP_FirstPersonCharacter OtherActor))
  (Development|SetHiddeninGame (Variables|Default|GetWidget) true false))

(event EventInteract
  (Utilities|IsValid (stale OnComponentEndOverlap(Box) _asbp_first_person_character)
    (:Is%20Valid
      (Variables|/Game/FirstPerson/Blueprints/BP_FirstPersonCharacter.BP_FirstPersonCharacter_C|SetHasEmeraldKey? (stale OnComponentEndOverlap(Box) _asbp_first_person_character) true)
      (Audio|PlaySound2D "/Game/Game/Audio/PlayerSounds/Key_Pickup.Key_Pickup" 1.0 1.0 0.0 0 0)
      (Actor|DestroyActor))
    (:Is%20Not%20Valid
      (bind _asbp_first_person_character (Utilities|Casting|CastToBP_FirstPersonCharacter (Game|GetPlayerCharacter 0)))
      (Variables|/Game/FirstPerson/Blueprints/BP_FirstPersonCharacter.BP_FirstPersonCharacter_C|SetHasEmeraldKey? _asbp_first_person_character true)
      (Audio|PlaySound2D "/Game/Game/Audio/PlayerSounds/Key_Pickup.Key_Pickup" 1.0 1.0 0.0 0 0)
      (Actor|DestroyActor))))

(fn ConstructionScript)