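; UnOpenableDoor_BP is an interactable door that cannot be opened.
; Its Interact event only plays the UnopenableDoor sound in 2D.
; A Box component's begin and end overlap events cast the other actor to the first-person character and four family enemy AI classes, but nothing follows the casts.
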(event OnComponentEndOverlap(Box)
  (params (OverlappedComponent :type Primitive%20Component%20Object%20Reference) (OtherActor :type Actor%20Object%20Reference) (OtherComp :type Primitive%20Component%20Object%20Reference) (OtherBodyIndex :type Integer))
  (Utilities|FlowControl|Sequence
    (:then_0
      (Utilities|Casting|CastToBP_FirstPersonCharacter OtherActor))
    (:then_1
      (Utilities|Casting|CastToBP_TheChildEnemyAI OtherActor))
    (:then_2
      (Utilities|Casting|CastToBP_TheDaughterEnemyAI OtherActor))
    (:then_3
      (Utilities|Casting|CastToBP_TheFatherEnemyAI OtherActor))
    (:then_4
      (Utilities|Casting|CastToBP_TheMotherEnemyAI OtherActor))))

(event OnComponentBeginOverlap(Box)
  (params (OverlappedComponent :type Primitive%20Component%20Object%20Reference) (OtherActor :type Actor%20Object%20Reference) (OtherComp :type Primitive%20Component%20Object%20Reference) (OtherBodyIndex :type Integer) (bFromSweep :type Boolean) (SweepResult :type Hit%20Result%20Structure%20%28by%20ref%29))
  (Utilities|FlowControl|Sequence
    (:then_0
      (Utilities|Casting|CastToBP_FirstPersonCharacter OtherActor))
    (:then_1
      (Utilities|Casting|CastToBP_TheChildEnemyAI OtherActor))
    (:then_2
      (Utilities|Casting|CastToBP_TheDaughterEnemyAI OtherActor))
    (:then_3
      (Utilities|Casting|CastToBP_TheFatherEnemyAI OtherActor))
    (:then_4
      (Utilities|Casting|CastToBP_TheMotherEnemyAI OtherActor))))

(event EventBeginPlay)

(event Collision|EventActorBeginOverlap
  (params (OtherActor :type Actor%20Object%20Reference)))

(event EventTick
  (params (DeltaSeconds :type Float%20%28single-precision%29)))

(event EventInteract
  (Audio|PlaySound2D "/Game/Game/Audio/UnopenableDoor.UnopenableDoor" 1.0 1.0 0.0 0 0))

(fn ConstructionScript)