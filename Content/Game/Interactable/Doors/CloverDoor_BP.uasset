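; An interactable door that opens only when the player character holds the Clover key.
; Entering the trigger box caches the player and shows a prompt widget, plus a second widget when the key is missing.
; Interact plays a locked sound or unlocks and drives a timeline that yaws the skeletal mesh up to 90 degrees.
; Leaving the box reverses the timeline, plays a closing sound if the door was open, and hides both widgets.
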(event OnComponentEndOverlap(Box)
  (params (OverlappedComponent :type Primitive%20Component%20Object%20Reference) (OtherActor :type Actor%20Object%20Reference) (OtherComp :type Primitive%20Component%20Object%20Reference) (OtherBodyIndex :type Integer))
  (Utilities|Casting|CastToBP_FirstPersonCharacter OtherActor)
  (Utilities|FlowControl|Sequence
    (:then_0
      (bind _doortimer (Timeline|DoorTimer Reverse)
        (:Update
          (Transformation|SetRelativeRotation (Variables|Default|GetSkeletalMesh) (Math|Rotator|MakeRotator 0.0 0.0 (* _doortimer 9e+01)) false false))))
    (:then_1
      (if (Variables|Default|GetDoorOpen?)
        (Audio|PlaySound2D "/Game/Game/Audio/Door_Closing.Door_Closing" 1.0 1.0 0.0 0 0)
        (Variables|Default|SetDoorOpen? false)
        (Timeline|DoorTimer Reverse)))
    (:then_2
      (Development|SetHiddeninGame (Variables|Default|GetWidget) true false))))

(event OnComponentBeginOverlap(Box)
  (params (OverlappedComponent :type Primitive%20Component%20Object%20Reference) (OtherActor :type Actor%20Object%20Reference) (OtherComp :type Primitive%20Component%20Object%20Reference) (OtherBodyIndex :type Integer) (bFromSweep :type Boolean) (SweepResult :type Hit%20Result%20Structure%20%28by%20ref%29))
  (bind _asbp_first_person_character (Utilities|Casting|CastToBP_FirstPersonCharacter OtherActor))
  (Development|SetHiddeninGame (Variables|Default|GetWidget) false false)
  (if (not (Variables|/Game/FirstPerson/Blueprints/BP_FirstPersonCharacter.BP_FirstPersonCharacter_C|GetHasCloverKey? _asbp_first_person_character))
    (Development|SetHiddeninGame (Variables|Default|GetWidget1) false false)))

(event EventBeginPlay)

(event Collision|EventActorBeginOverlap
  (params (OtherActor :type Actor%20Object%20Reference)))

(event EventTick
  (params (DeltaSeconds :type Float%20%28single-precision%29)))

(event EventInteract
  (if (Variables|/Game/FirstPerson/Blueprints/BP_FirstPersonCharacter.BP_FirstPersonCharacter_C|GetHasCloverKey? (stale OnComponentBeginOverlap(Box) _asbp_first_person_character))
    (Audio|PlaySound2D "/Game/Game/Audio/Door_Unlocked.Door_Unlocked" 1.0 1.0 0.0 0 0)
    (Variables|Default|SetDoorOpen? true)
    (bind _doortimer (Timeline|DoorTimer Play)
      (:Update
        (Transformation|SetRelativeRotation (Variables|Default|GetSkeletalMesh) (Math|Rotator|MakeRotator 0.0 0.0 (* _doortimer 9e+01)) false false)))
    (else
      (Audio|PlaySound2D "/Game/Game/Audio/Door_Locked.Door_Locked" 1.0 1.0 0.0 0 0))))

(fn ConstructionScript)