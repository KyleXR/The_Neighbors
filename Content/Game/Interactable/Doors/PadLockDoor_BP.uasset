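; PadLockDoor_BP is an interactable door that stays locked until the player enters the correct PIN.
; Interact toggles a W_Padlock keypad widget and cursor input mode while locked, or swings the mesh open via the DoorTimer timeline once unlocked.
; AddToPin checks the widget's input against Pin to unlock or show an error.
; Box overlap shows the prompt widget and closes the door when the player leaves; enemy overlap branches are empty.
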(event OnComponentEndOverlap(Box)
  (params (OverlappedComponent :type Primitive%20Component%20Object%20Reference) (OtherActor :type Actor%20Object%20Reference) (OtherComp :type Primitive%20Component%20Object%20Reference) (OtherBodyIndex :type Integer))
  (Utilities|FlowControl|Sequence
    (:then_0
      (Utilities|Casting|CastToBP_FirstPersonCharacter OtherActor)
      (Utilities|FlowControl|Sequence
        (:then_0
          (bind _doortimer (Timeline|DoorTimer Reverse)
            (:Update
              (Transformation|SetRelativeRotation (Variables|Default|GetSkeletalMesh) (Math|Rotator|MakeRotator 0.0 0.0 (* _doortimer 9e+01)) false false))))
        (:then_1
          (Development|SetHiddeninGame (Variables|Default|GetWidget) true false))
        (:then_2
          (if (Variables|Default|GetDoorOpen?)
            (Audio|PlaySound2D "/Game/Game/Audio/Door_Closing.Door_Closing" 1.0 1.0 0.0 0 0)
            (Variables|Default|SetDoorOpen? false)
            (Timeline|DoorTimer Reverse)))))
    (:then_1
      (Utilities|Casting|CastToBP_TheChildEnemyAI OtherActor))))

(event OnComponentBeginOverlap(Box)
  (params (OverlappedComponent :type Primitive%20Component%20Object%20Reference) (OtherActor :type Actor%20Object%20Reference) (OtherComp :type Primitive%20Component%20Object%20Reference) (OtherBodyIndex :type Integer) (bFromSweep :type Boolean) (SweepResult :type Hit%20Result%20Structure%20%28by%20ref%29))
  (Utilities|FlowControl|Sequence
    (:then_0
      (Utilities|Casting|CastToBP_FirstPersonCharacter OtherActor)
      (Development|SetHiddeninGame (Variables|Default|GetWidget) false false))
    (:then_1
      (Utilities|Casting|CastToBP_TheChildEnemyAI OtherActor))))

(event EventBeginPlay)

(event Collision|EventActorBeginOverlap
  (params (OtherActor :type Actor%20Object%20Reference)))

(event EventInteract
  (bind _returnvalue (Game|GetPlayerController 0))
  (bind _returnvalue_2 (Game|GetPlayerController 0))
  (if (Variables|Default|GetUnlocked)
    (Audio|PlaySound2D "/Game/Game/Audio/Door_Open.Door_Open" 1.0 1.0 0.0 0 0)
    (Variables|Default|SetDoorOpen? true)
    (bind _doortimer (Timeline|DoorTimer Play)
      (:Update
        (Transformation|SetRelativeRotation (Variables|Default|GetSkeletalMesh) (Math|Rotator|MakeRotator 0.0 0.0 (* _doortimer 9e+01)) false false)))
    (else
      (Utilities|IsValid (Variables|Default|GetPinWidgetREF)
        (:Is%20Valid
          (Widget|RemovefromParent (stale _output_get))
          (Variables|Default|SetPinWidgetREF 0)
          (Input|SetInputModeGameOnly _returnvalue false)
          (Variables|/Script/Engine.PlayerController|SetbShowMouseCursor _returnvalue false))
        (:Is%20Not%20Valid
          (bind _returnvalue_3 (UserInterface|CreateWidget "/Game/Game/Widgets/Menus/W_Padlock.W_Padlock_C" 0 self))
          (bind _output_get (Variables|Default|SetPinWidgetREF _returnvalue_3))
          (UserInterface|Viewport|AddtoViewport _output_get 0)
          (Input|SetInputModeGameandUI _returnvalue_2 _output_get "DoNotLock" false false)
          (Variables|/Script/Engine.PlayerController|SetbShowMouseCursor _returnvalue_2 true))))))

(fn ConstructionScript)

(fn AddtoPin
  (params (Input :type String))
  (bind _returnvalue (Game|GetPlayerController 0))
  (bind _pinwidgetref (Variables|Default|GetPinWidgetREF))
  (bind _pinwidgetref_2 (Variables|Default|GetPinWidgetREF))
  (if (Utilities|Enum|Equal(Enum) Input (Variables|Default|GetPin))
    (bind _output_get (Variables|/Game/Game/Widgets/Menus/W_Padlock.W_Padlock_C|SetInput _pinwidgetref "CORRECT"))
    (Rendering|Components|TextRender|SetText (Variables|/Game/Game/Widgets/Menus/W_Padlock.W_Padlock_C|GetW_Input _pinwidgetref) (Utilities|Text|ToText(String) _output_get))
    (Variables|Default|SetUnlocked true)
    (Widget|RemovefromParent _pinwidgetref)
    (Input|SetInputModeGameOnly _returnvalue false)
    (Variables|/Script/Engine.PlayerController|SetbShowMouseCursor _returnvalue false)
    (else
      (bind _output_get_2 (Variables|/Game/Game/Widgets/Menus/W_Padlock.W_Padlock_C|SetInput _pinwidgetref_2 "INCORRECT"))
      (Rendering|Components|TextRender|SetText (Variables|/Game/Game/Widgets/Menus/W_Padlock.W_Padlock_C|GetW_Input _pinwidgetref_2) (Utilities|Text|ToText(String) _output_get_2))
      (Default|DelayClear _pinwidgetref_2))))