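; Readable ruby key letter pickup that the player toggles open and closed through Interact.
; A box overlap stores the first-person character and shows a prompt widget; leaving hides it and closes the letter.
; Interact plays a pickup sound, swaps the world letter and prompt for a W_RubyKeyLetter screen widget, and hides the player actor while reading.
; Overlap casts to the four family enemy AIs lead nowhere.
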(event OnComponentBeginOverlap(Box)
  (params (OverlappedComponent :type Primitive%20Component%20Object%20Reference) (OtherActor :type Actor%20Object%20Reference) (OtherComp :type Primitive%20Component%20Object%20Reference) (OtherBodyIndex :type Integer) (bFromSweep :type Boolean) (SweepResult :type Hit%20Result%20Structure%20%28by%20ref%29))
  (Utilities|FlowControl|Sequence
    (:then_0
      (bind _asbp_first_person_character (Utilities|Casting|CastToBP_FirstPersonCharacter OtherActor))
      (Development|SetHiddeninGame (Variables|Default|GetWidget) false false))
    (:then_1
      (Utilities|Casting|CastToBP_TheChildEnemyAI OtherActor))
    (:then_2
      (Utilities|Casting|CastToBP_TheDaughterEnemyAI OtherActor))
    (:then_3
      (Utilities|Casting|CastToBP_TheFatherEnemyAI OtherActor))
    (:then_4
      (Utilities|Casting|CastToBP_TheMotherEnemyAI OtherActor))))

(event OnComponentEndOverlap(Box)
  (params (OverlappedComponent :type Primitive%20Component%20Object%20Reference) (OtherActor :type Actor%20Object%20Reference) (OtherComp :type Primitive%20Component%20Object%20Reference) (OtherBodyIndex :type Integer))
  (Utilities|FlowControl|Sequence
    (:then_0
      (Utilities|Casting|CastToBP_FirstPersonCharacter OtherActor)
      (Development|SetHiddeninGame (Variables|Default|GetWidget) true false)
      (Variables|Default|SetIsHoldingLetter? false)
      (Widget|RemovefromParent (stale EventInteract _returnvalue)))
    (:then_1
      (Utilities|Casting|CastToBP_TheChildEnemyAI OtherActor))
    (:then_2
      (Utilities|Casting|CastToBP_TheDaughterEnemyAI OtherActor))
    (:then_3
      (Utilities|Casting|CastToBP_TheFatherEnemyAI OtherActor))
    (:then_4
      (Utilities|Casting|CastToBP_TheMotherEnemyAI OtherActor))))

(event EventInteract
  (Audio|PlaySound2D "/Game/Game/Audio/PickupLetter.PickupLetter" 1.0 1.0 0.0 0 0)
  (if (Variables|Default|GetIsHoldingLetter?)
    (Variables|Default|SetIsHoldingLetter? false)
    (Development|SetHiddeninGame (Variables|Default|GetLetter) false false)
    (Widget|RemovefromParent (stale _returnvalue))
    (Rendering|SetActorHiddenInGame (stale OnComponentBeginOverlap(Box) _asbp_first_person_character) false)
    (else
      (Variables|Default|SetIsHoldingLetter? true)
      (Development|SetHiddeninGame (Variables|Default|GetLetter) true false)
      (bind _returnvalue (UserInterface|CreateWidget "/Game/Game/Widgets/Letters/Letters/W_RubyKeyLetter.W_RubyKeyLetter_C"))
      (UserInterface|Viewport|AddtoViewport _returnvalue 0)
      (Rendering|SetActorHiddenInGame (stale OnComponentBeginOverlap(Box) _asbp_first_person_character) true))))

(fn ConstructionScript
  (|CallParentFunction))